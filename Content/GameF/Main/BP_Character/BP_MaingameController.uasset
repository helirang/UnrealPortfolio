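; BP_MaingameController is the main game's player controller, handling input setup and the ending sequence.
; On BeginPlay it hides the cursor and sets game-only input, and DeleteWidget clears all widgets.
; EndSetting clears widgets, cuts to a start view target and slowly blends to an end target as a camera move.
; After a delay outlasting the blend, it shows BP_EndingWidget and the mouse cursor.
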(event Custom|DeleteWidget
  (Viewport|RemoveAllWidgets))

(event Custom|EndSetting
  (params (EndViewTarget :type Camera%20Actor%20Object%20Reference) (StartViewTarget :type Camera%20Actor%20Object%20Reference))
  (Viewport|RemoveAllWidgets)
  (Game|Player|SetViewTargetwithBlend StartViewTarget 0.0 "VTBlend_Linear" 0.0 false)
  (Game|Player|SetViewTargetwithBlend EndViewTarget 12.0 "VTBlend_Linear" 0.0 false)
  (Utilities|FlowControl|Delay 16.0)
  (bind _returnvalue (UserInterface|CreateWidget "/Game/GameF/Main/BP_Character/UI/BP_EndingWidget.BP_EndingWidget_C" self))
  (Utilities|IsValid _returnvalue
    (:Is%20Valid
      (UserInterface|Viewport|AddtoViewport _returnvalue 0)
      (Variables|Default|SetbShowMouseCursor true))))

(event EventBeginPlay
  (Variables|Default|SetbShowMouseCursor false)
  (Input|SetInputModeGameOnly self))

(event EventTick
  (params (DeltaSeconds :type Float%20%28single-precision%29)))

(fn ConstructionScript)