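; Player character Blueprint that creates the gameplay HUD widget for the locally controlled player and handles spawn and death presentation.
; Tick drives a material-based appear/disappear effect, animating a Radius parameter around an InOutPosition below the actor, disappearing on death or game end.
; Death disables selected collision responses, stops firing and sets a lifespan, while respawn requests go through MainGamePlayerState.
; Weapon-socket camera zoom is a failed experiment left unwired.
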(event EventBeginPlay
  (if (Pawn|IsLocallyControlled)
    (bind _returnvalue (UserInterface|CreateWidget "/Game/GameF/Main/BP_Character/UI/BP_UserGamePlayWidget.BP_UserGamePlayWidget_C"))
    (UserInterface|Viewport|AddtoViewport _returnvalue 0)))

(event EventReSpawnRequest
  (bind _asmain_game_player_state (Utilities|Casting|CastToMainGamePlayerState (Variables|Default|GetPlayerState)))
  (bind _asplayer_controller (Utilities|Casting|CastToPlayerController (Pawn|GetController)))
  (Class|MainGamePlayerState|ClientRequest _asmain_game_player_state _asplayer_controller))

(event EventTick
  (params (DeltaSeconds :type Float%20%28single-precision%29))
  (if (Variables|Default|GetbAppearOrDisAppear)
    (if (Variables|Default|GetbEndGame)
      (CallFunction|DisappearCharacter DeltaSeconds)
      (elif (Variables|Default|GetbDied)
        (CallFunction|DisappearCharacter DeltaSeconds)
        (else
          (CallFunction|AppearCharacter DeltaSeconds))))))

(event EventZoomLocationChange
  (bind _currentweapon (Variables|Default|GetCurrentWeapon))
  ;[1 1 1] 줌 테스트 실퓨ㅐ
  (Utilities|IsValid _currentweapon
    (:Is%20Valid
      (Transformation|SetWorldLocation (Variables|Default|GetCameraComp) (Transformation|GetSocketLocation (Variables|/Script/CodeGameAlpha.OriginWeapon|GetMeshComp _currentweapon) "ZoomSocket") false false))))

(fn ConstructionScript)

(fn AppearCharacter
  (params (DeltaSecond :type Float%20%28single-precision%29))
  (if (Variables|Default|GetbAppearCharacter)
    (Rendering|Material|SetVectorParameterValueonMaterials (Variables|Character|GetMesh) "InOutPosition" (- (Transformation|GetActorLocation) "0, 0,150.000000"))
    (Variables|Default|SetbAppearCharacter false)
    (else
      (bind _output_get (Variables|Default|SetRadius (- (Variables|Default|GetRadius) (* DeltaSecond (Variables|Default|GetFrameRadius)))))))
  (Rendering|Material|SetScalarParameterValueonMaterials (Variables|Character|GetMesh) "Radius" _output_get)
  (if (not (>= (Variables|Default|GetRadius) 0.0))
    (bind _output_get_2 (Variables|Default|SetRadius 0.0))
    (Rendering|Material|SetScalarParameterValueonMaterials (Variables|Character|GetMesh) "Radius" _output_get_2)
    (Variables|Default|SetbAppearOrDisAppear false)))

(fn DisappearCharacter
  (params (DeltaSecond :type Float%20%28single-precision%29))
  (if (Variables|Default|GetbDisappearStart)
    (Variables|Default|SetFrameRadius 1.3e+02)
    (Variables|Default|SetbDisappearStart false)
    (Rendering|Material|SetVectorParameterValueonMaterials (Variables|Character|GetMesh) "InOutPosition" (- (Transformation|GetActorLocation) "0, 0,150.000000")))
  (bind _output_get (Variables|Default|SetRadius (+ (Variables|Default|GetRadius) (* DeltaSecond (Variables|Default|GetFrameRadius)))))
  (Rendering|Material|SetScalarParameterValueonMaterials (Variables|Character|GetMesh) "Radius" _output_get)
  (if (not (<= (Variables|Default|GetRadius) 1e+03))
    (bind _output_get_2 (Variables|Default|SetRadius 8e+02))
    (Rendering|Material|SetScalarParameterValueonMaterials (Variables|Character|GetMesh) "Radius" _output_get_2)
    (Variables|Default|SetbAppearOrDisAppear false)))

(fn CharacterDiedCallFunc
  (bind _capsulecomponent (Variables|Default|GetCapsuleComponent))
  (Collision|SetCollisionResponsetoChannel _capsulecomponent "ECC_Pawn" "ECR_Ignore")
  (Collision|SetCollisionResponsetoChannel _capsulecomponent "ECC_Camera" "ECR_Ignore")
  (Collision|SetCollisionResponsetoChannel (Variables|Character|GetMesh) "ECC_GameTraceChannel1" "ECR_Ignore")
  (Class|MainCharacter|StopFire)
  (Actor|SetLifeSpan 5.0))