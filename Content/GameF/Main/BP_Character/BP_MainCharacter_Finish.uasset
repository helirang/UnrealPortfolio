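; Main character Blueprint for a networked shooter, handling local HUD creation, spawn audio based on death score, respawn requests and death cleanup.
; Tick animates a material-driven appear/disappear effect through a growing or shrinking radius, using world offset.
; On the server, Tick also computes aim pitch from the weapon muzzle toward the view target.
; Firing plays rifle audio and, with authority, reports noise for AI hearing.
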(event EventFireAddReportNoiseEvent
  (bind _characteraudiocomp (Variables|Default|GetCharacterAudioComp))
  ;[1 1 1] AI Hearing 작동 Noise 생성
  (Effects|Components|ParticleSystem|SetIntParameter _characteraudiocomp "RifleSound" 0)
  (Audio|Components|Audio|Play _characteraudiocomp 0.0)
  (Networking|SwitchHasAuthority
    (:Authority
      (Class|AISenseHearing|ReportNoiseEvent (Transformation|GetActorLocation) 1.0 self 1.5e+03 "Noise"))))

(event EventReSpawnRequest
  ;[1 1 1] 서버로 리스폰 요청 ( PlayerState에 구현 )
  (bind _asmain_game_player_state (Utilities|Casting|CastToMainGamePlayerState (Variables|Default|GetPlayerState)))
  (bind _asplayer_controller (Utilities|Casting|CastToPlayerController (Pawn|GetController)))
  (if (Networking|IsServer)
    (Class|MainGamePlayerState|ClientRequest _asmain_game_player_state _asplayer_controller)
    (Development|PrintString "server")
    (else
      (Development|PrintString "NotServer"))))

(event EventBeginPlay
  ;[1 1 1] UI
  (CallFunction|PlayPossesandBeginPlay)
  (if (Pawn|IsLocallyControlled)
    (Networking|SwitchHasAuthority
      (:Remote
        (bind _returnvalue (UserInterface|CreateWidget "/Game/GameF/Main/BP_Character/UI/BP_UserGamePlayWidget.BP_UserGamePlayWidget_C"))
        (UserInterface|Viewport|AddtoViewport _returnvalue 0)
        (Networking|SwitchHasAuthority)))
    (else
      (Development|PrintString "not work"))))

(event EventTick
  (params (DeltaSeconds :type Float%20%28single-precision%29))
  (bind (_outlocation _outrotation) (Actor|GetActorEyesViewPoint))
  (bind _self self)
  (bind _currentweapon (Variables|/Script/CodeGameAlpha.MainCharacter|GetCurrentWeapon _self))
  (Utilities|FlowControl|Sequence
    (:then_0
      ;[1 1 1] 캐릭터 등장, 퇴장 효과 ( 메테리얼 월드 오프셋 사용 )
      (if (Variables|Default|GetbAppearOrDisAppear)
        (if (Variables|Default|GetbEndGame)
          (CallFunction|DisappearCharacter DeltaSeconds)
          (elif (Variables|Default|GetbDied)
            (CallFunction|DisappearCharacter DeltaSeconds)
            (else
              (CallFunction|AppearCharacter DeltaSeconds))))))
    (:then_1
      ;[1 1 1] Player 총구 정렬
      (Networking|SwitchHasAuthority
        (:Authority
          (Utilities|IsValid _currentweapon
            (:Is%20Valid
              (Variables|Default|SetPitch (+ (.pitch (Transformation|GetActorRotation)) (.pitch (Math|Rotator|FindLookatRotation (Transformation|GetSocketLocation (Variables|/Script/CodeGameAlpha.OriginWeapon|GetMeshComp _currentweapon) "MuzzleSocket") (+ _outlocation (* (Math|Rotator|GetRotationXVector _outrotation) 1e+04)))))))))))))

(event EventPossessed
  (params (NewController :type Controller%20Object%20Reference))
  ;[1 1 1] UI
  (Networking|SwitchHasAuthority
    (:Authority
      (if (Pawn|IsLocallyControlled)
        (CallFunction|PlayPossesandBeginPlay)
        (bind _returnvalue (UserInterface|CreateWidget "/Game/GameF/Main/BP_Character/UI/BP_UserGamePlayWidget.BP_UserGamePlayWidget_C"))
        (UserInterface|Viewport|AddtoViewport _returnvalue 0)))))

(fn ConstructionScript)

(fn AppearCharacter
  (params (DeltaSecond :type Float%20%28single-precision%29))
  (if (Variables|Default|GetbAppearCharacter)
    (Rendering|Material|SetVectorParameterValueonMaterials (Variables|Character|GetMesh) "InOutPosition" (- (Transformation|GetActorLocation) "0, 0,150.000000"))
    (Variables|Default|SetbAppearCharacter false)
    (else
      (bind _output_get (Variables|Default|SetRadius (- (Variables|Default|GetRadius) (* DeltaSecond (Variables|Default|GetFrameRadius)))))))
  (Rendering|Material|SetScalarParameterValueonMaterials (Variables|Character|GetMesh) "Radius" _output_get)
  (if (not (>= (Variables|Default|GetRadius) 0.0))
    (bind _output_get_2 (Variables|Default|SetRadius 0.0))
    (Rendering|Material|SetScalarParameterValueonMaterials (Variables|Character|GetMesh) "Radius" _output_get_2)
    (Variables|Default|SetbAppearOrDisAppear false)))

(fn DisappearCharacter
  (params (DeltaSecond :type Float%20%28single-precision%29))
  (if (Variables|Default|GetbDisappearStart)
    (Variables|Default|SetFrameRadius 1.3e+02)
    (Variables|Default|SetbDisappearStart false)
    (Rendering|Material|SetVectorParameterValueonMaterials (Variables|Character|GetMesh) "InOutPosition" (- (Transformation|GetActorLocation) "0.000000,0.000000,150.000000")))
  (bind _output_get (Variables|Default|SetRadius (+ (Variables|Default|GetRadius) (* DeltaSecond (Variables|Default|GetFrameRadius)))))
  (Rendering|Material|SetScalarParameterValueonMaterials (Variables|Character|GetMesh) "Radius" _output_get)
  (if (not (<= (Variables|Default|GetRadius) 1e+03))
    (bind _output_get_2 (Variables|Default|SetRadius 8e+02))
    (Rendering|Material|SetScalarParameterValueonMaterials (Variables|Character|GetMesh) "Radius" _output_get_2)
    (Variables|Default|SetbAppearOrDisAppear false)))

(fn CharacterDiedCallFunc
  (bind _capsulecomponent (Variables|Default|GetCapsuleComponent))
  (Collision|SetCollisionResponsetoChannel _capsulecomponent "ECC_Pawn" "ECR_Ignore")
  (Collision|SetCollisionResponsetoChannel _capsulecomponent "ECC_Camera" "ECR_Ignore")
  (Collision|SetCollisionResponsetoChannel (Variables|Character|GetMesh) "ECC_GameTraceChannel1" "ECR_Ignore")
  (Class|MainCharacter|StopFire)
  (Actor|SetLifeSpan 5.0))

(fn PlayPossesandBeginPlay
  (bind _characteraudiocomp3 (Variables|Default|GetCharacterAudioComp3))
  (if (not (Variables|Default|GetbBot))
    (bind _asps_main_game_player_state (Utilities|Casting|CastToPS_MainGamePlayerState (Variables|Default|GetPlayerState)))
    (bind _returnvalue (Class|MainGamePlayerState|NowDeadScore _asps_main_game_player_state))
    (if (> _returnvalue 0)
      (Effects|Components|ParticleSystem|SetIntParameter _characteraudiocomp3 "CharacterSound" 2)
      (else
        (Effects|Components|ParticleSystem|SetIntParameter _characteraudiocomp3 "CharacterSound" 1)))
    (Audio|Components|Audio|Play _characteraudiocomp3 0.0)))