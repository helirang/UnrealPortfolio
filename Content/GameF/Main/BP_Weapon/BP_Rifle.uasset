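; Rifle weapon Blueprint that adds a material-driven appear effect and reports bullet impact noise.
; While TickAppear is set, Tick anchors the effect's InOutPosition below the owner once, then shrinks the mesh materials' Radius over time until it reaches zero.
; Impact points raise a short-range "BulletNoise" noise event instigated by the owning MainCharacter, only when that character is not a bot.
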(event EventReportNoiseImpactPoint
  (params (NoiseLocation :type Vector :default "0, 0, 0"))
  (bind _returnvalue (Components|GetOwner))
  (Utilities|IsValid _returnvalue
    (:Is%20Valid
      (bind _asmain_character (Utilities|Casting|CastToMainCharacter _returnvalue))
      (if (not (Variables|/Script/CodeGameAlpha.MainCharacter|GetbBot _asmain_character))
        (Class|AISenseHearing|ReportNoiseEvent NoiseLocation 1.0 _asmain_character 5e+02 "BulletNoise")))))

(event EventTick
  (params (DeltaSeconds :type Float%20%28single-precision%29))
  (if (Variables|Default|GetTickAppear)
    (if (Variables|Default|GetAppear)
      (Rendering|Material|SetVectorParameterValueonMaterials (Variables|Default|GetMeshComp) "InOutPosition" (- (Transformation|GetActorLocation (Components|GetOwner)) "0, 0,150.000000"))
      (Variables|Default|SetAppear false))
    (bind _output_get (Variables|Default|SetRidius (- (Variables|Default|GetRidius) (* DeltaSeconds (Variables|Default|GetFrameRadius)))))
    (Rendering|Material|SetScalarParameterValueonMaterials (Variables|Default|GetMeshComp) "Radius" _output_get)
    (if (not (>= (Variables|Default|GetRidius) 0.0))
      (bind _output_get_2 (Variables|Default|SetRidius 0.0))
      (Rendering|Material|SetScalarParameterValueonMaterials (Variables|Default|GetMeshComp) "Radius" _output_get_2)
      (Variables|Default|SetTickAppear false))))

(fn ConstructionScript)