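; BP_Bot_Rifle is a bot's rifle weapon that plays a material-driven appear and disappear effect.
; While TickAppear is set, Tick anchors InOutPosition below the owner and shrinks the Radius parameter to zero.
; Afterward, once the BP_Bot owner has died and DisAppearFirst is set, it re-anchors and grows the radius.
; GetBotFireDirection only draws a debug line from a MainCharacter owner toward TargetActor and returns zero.
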(event EventBeginPlay)

(event EventTick
  (params (DeltaSeconds :type Float%20%28single-precision%29))
  (if (Variables|Default|GetTickAppear)
    (if (Variables|Default|GetAppear)
      (Rendering|Material|SetVectorParameterValueonMaterials (Variables|Default|GetMeshComp) "InOutPosition" (- (Transformation|GetActorLocation (Components|GetOwner)) "0, 0,150.000000"))
      (Variables|Default|SetAppear false))
    (bind _output_get (Variables|Default|SetRidius (- (Variables|Default|GetRidius) (* DeltaSeconds (Variables|Default|GetFrameRadius)))))
    (Rendering|Material|SetScalarParameterValueonMaterials (Variables|Default|GetMeshComp) "Radius" _output_get)
    (if (not (>= (Variables|Default|GetRidius) 0.0))
      (bind _output_get_2 (Variables|Default|SetRidius 0.0))
      (Rendering|Material|SetScalarParameterValueonMaterials (Variables|Default|GetMeshComp) "Radius" _output_get_2)
      (Variables|Default|SetTickAppear false))
    (else
      (bind _asbp_bot (Utilities|Casting|CastToBP_Bot (Components|GetOwner)))
      (if (Variables|/Script/CodeGameAlpha.MainCharacter|GetbDied _asbp_bot)
        (if (Variables|Default|GetbDisAppearFirst)
          (if (Variables|Default|GetbDisAppear)
            (Rendering|Material|SetVectorParameterValueonMaterials (Variables|Default|GetMeshComp) "InOutPosition" (- (Transformation|GetActorLocation _asbp_bot) "0, 0,150.000000"))
            (Variables|Default|SetbDisAppear false)
            (Variables|Default|SetFrameRadius 1.3e+02))
          (bind _output_get_3 (Variables|Default|SetRidius (+ (Variables|Default|GetRidius) (* DeltaSeconds (Variables|Default|GetFrameRadius)))))
          (Rendering|Material|SetScalarParameterValueonMaterials (Variables|Default|GetMeshComp) "Radius" _output_get_3)
          (if (not (<= (Variables|Default|GetRidius) 1e+03))
            (bind _output_get_4 (Variables|Default|SetRidius 8e+02))
            (Rendering|Material|SetScalarParameterValueonMaterials (Variables|Default|GetMeshComp) "Radius" _output_get_4)
            (Variables|Default|SetbDisAppear false)))))))

(fn ConstructionScript)

(fn GetBotFireDirection
  (bind _returnvalue (Components|GetOwner))
  (bind _targetactor (Variables|Default|GetTargetActor))
  (Utilities|IsValid _targetactor
    (:Is%20Valid
      (Utilities|IsValid _returnvalue
        (:Is%20Valid
          (bind _asmain_character (Utilities|Casting|CastToMainCharacter _returnvalue))
          (Rendering|Debug|DrawDebugLine :LineStart (Transformation|GetActorLocation _asmain_character) :LineEnd (+ (.location (Math|Transform|MakeTransform (Transformation|GetActorLocation _asmain_character) (Math|Rotator|FindLookatRotation (+ (Transformation|GetActorLocation _asmain_character) (Transformation|GetActorForwardVector _asmain_character)) (Transformation|GetActorLocation _targetactor)))) (* (Math|Vector|GetForwardVector (Math|Rotator|FindLookatRotation (+ (Transformation|GetActorLocation _asmain_character) (Transformation|GetActorForwardVector _asmain_character)) (Transformation|GetActorLocation _targetactor))) 3e+02)) :Duration 1e+01 :Thickness 1.0)
          (return 0.0))))))