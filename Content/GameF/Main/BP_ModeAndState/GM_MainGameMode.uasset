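; GM_MainGameMode is the main game mode, handling bot spawning and end-of-game cleanup for the player and bots.
; SpawnBot waits one second, then spawns a BP_Bot at every TargetPoint in the level.
; GameEnding and AllKillAI set the disappear and end-game flags on the given controller's BP_MainCharacter_Finish pawn or on all bots, then trigger a timed ClearDeath.
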(event Custom|AllKillAI
  ;[1 1 1] 모든 봇 사망처리
  (bind _outactors (Actor|GetAllActorsOfClass "/Game/GameF/Main/BP_Character/BP_Bot.BP_Bot_C"))
  (for _array_element _outactors
    (Variables|/Script/CodeGameAlpha.MainCharacter|SetbAppearOrDisAppear _array_element true)
    (Variables|/Game/GameF/Main/BP_Character/BP_Bot.BP_Bot_C|SetbEndGame _array_element true)
    (Class|MainCharacter|ClearDeath _array_element 5.0)))

(event Custom|SpawnBot
  ;[1 1 1] 봇 스폰
  (bind _outactors (Actor|GetAllActorsOfClass "/Script/Engine.TargetPoint"))
  (Utilities|FlowControl|Delay 1.0)
  (for _array_element _outactors
    (Game|SpawnActorfromClass "/Game/GameF/Main/BP_Character/BP_Bot.BP_Bot_C" (Math|Transform|MakeTransform (Transformation|GetActorLocation _array_element) "0,180.000000, 0") "AdjustIfPossibleButDontSpawnIfColliding" 0 0) ; spawn actor from class
  ))

(event EventTick
  (params (DeltaSeconds :type Float%20%28single-precision%29)))

(event EventGameEnding
  (params (PC :type Player%20Controller%20Object%20Reference) (CA :type Camera%20Actor%20Object%20Reference))
  (bind _returnvalue (Pawn|GetControlledPawn PC))
  ;[1 1 1] 유저 Pawn 사망 처리 및 퇴장효과 작동
  (Utilities|IsValid _returnvalue
    (:Is%20Valid
      (bind _asbp_main_character_finish (Utilities|Casting|CastToBP_MainCharacter_Finish _returnvalue))
      (Variables|/Script/CodeGameAlpha.MainCharacter|SetbAppearOrDisAppear _asbp_main_character_finish true)
      (Variables|/Game/GameF/Main/BP_Character/BP_MainCharacter_Finish.BP_MainCharacter_Finish_C|SetbEndGame _asbp_main_character_finish true)
      (Class|MainCharacter|ClearDeath _asbp_main_character_finish 5.0))))

(fn ConstructionScript)